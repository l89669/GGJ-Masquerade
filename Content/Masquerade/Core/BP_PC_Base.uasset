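; Base player controller that provides global input, the eye-blink screen effect and level-unlock tracking.
; On BeginPlay it adds the global mapping context, creates a top-layer blink widget and marks the current level as opened in the GameInstance's level list.
; Eye open and close events drive the MPC_Blink Progress parameter through a reversible timeline, either continuing or restarting.
; Enhanced Input actions open the ESC menu or quit the game.
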(event Custom|OpenEye
  (params (continue :type Boolean))
  ;[0.15 0.15 0.15 0.5] 眨眼特效（在LV_CG和LV_1都要用，只能放这里）
  (if continue
    (bind _alpha (Timeline|时间轴 Play)
      (:Update
        (Rendering|Material|SetScalarParameterValue "/Game/Masquerade/UI/MPC_Blink.MPC_Blink" "Progress" _alpha :!class /Script/Engine.KismetMaterialLibrary)))
    (else
      (Rendering|Material|SetScalarParameterValue "/Game/Masquerade/UI/MPC_Blink.MPC_Blink" "Progress" 0.0 :!class /Script/Engine.KismetMaterialLibrary)
      (Timeline|时间轴 PlayFromStart))))

(event Custom|CloseEye
  (params (continue :type Boolean))
  ;[0.15 0.15 0.15 0.5] 眨眼特效（在LV_CG和LV_1都要用，只能放这里）
  (if continue
    (bind _alpha (Timeline|时间轴 Reverse)
      (:Update
        (Rendering|Material|SetScalarParameterValue "/Game/Masquerade/UI/MPC_Blink.MPC_Blink" "Progress" _alpha :!class /Script/Engine.KismetMaterialLibrary)))
    (else
      (Rendering|Material|SetScalarParameterValue "/Game/Masquerade/UI/MPC_Blink.MPC_Blink" "Progress" 1.0 :!class /Script/Engine.KismetMaterialLibrary)
      (Timeline|时间轴 ReverseFromEnd))))

(event Custom|SetEyeState
  (params (Open :type Boolean))
  ;[0.15 0.15 0.15 0.5] 眨眼特效（在LV_CG和LV_1都要用，只能放这里）
  (Rendering|Material|SetScalarParameterValue "/Game/Masquerade/UI/MPC_Blink.MPC_Blink" "Progress" (Math|Float|SelectFloat 1.0 0.0 Open) :!class /Script/Engine.KismetMaterialLibrary))

(event Input|EnhancedActionEvents|EnhancedInputActionIA_ESC
  (params (ActionValue :type Boolean) (ElapsedSeconds :type Float%20%28double-precision%29) (TriggeredSeconds :type Float%20%28double-precision%29) (InputAction :type Input%20Action%20Object%20Reference :default "/Game/Masquerade/Characters/Player/Input/Actions/IA_ESC.IA_ESC"))
  ;[0.15 0.15 0.15 0.5] ESC菜单
  (:Started
    (bind _returnvalue (UserInterface|CreateWidget "/Game/Masquerade/UI/WBP_ESC.WBP_ESC_C" self))
    (UserInterface|Viewport|AddtoViewport _returnvalue 0)))

(event Input|EnhancedActionEvents|EnhancedInputActionIA_Quit
  (params (ActionValue :type Boolean) (ElapsedSeconds :type Float%20%28double-precision%29) (TriggeredSeconds :type Float%20%28double-precision%29) (InputAction :type Input%20Action%20Object%20Reference :default "/Game/Masquerade/Characters/Player/Input/Actions/IA_Quit.IA_Quit"))
  ;[0.15 0 0 0.5] 退出游戏
  (:Started
    (Game|QuitGame self "Quit" false)))

(event EventBeginPlay
  (bind _game_instance (CallFunction|GetGameInstance))
  (bind _returnvalue (PlayerController|LocalPlayerSubsystems|GetEnhancedInputLocalPlayerSubsystem))
  (bind _level_names (Variables|/Game/Masquerade/Core/BP_GI_Base.BP_GI_Base_C|GetLevel%20Names _game_instance))
  ;[0.15 0.15 0.15 0.5] 眨眼特效（在LV_CG和LV_1都要用，只能放这里）
  (Utilities|FlowControl|Sequence
    (:then_0
      ;[0.15 0.15 0.15 0.5] 添加映射上下文
      (Utilities|IsValid _returnvalue
        (:Is%20Valid
          (Input|AddMappingContext _returnvalue "/Game/Masquerade/Characters/Player/Input/IMC_Global.IMC_Global" 0 "(bIgnoreAllPressedKeysUntilRelease=True,bForceImmediately=False,bNotifyUserSettings=False)"))))
    (:then_1
      (bind _returnvalue_2 (UserInterface|CreateWidget "/Game/Masquerade/UI/WBP_BlinkLayer.WBP_BlinkLayer_C" self))
      (UserInterface|Viewport|AddtoViewport _returnvalue_2 10000)
      (CallFunction|SetEyeState true))
    (:then_2
      ;[0.15 0.15 0.15 0.5] 每次解锁新关卡时记录为解锁
      (for (_array_element _array_index) _level_names
        (bind _returnvalue_3 (Game|GetCurrentLevelName true))
        (if (== (.LevelName (Utilities|Struct|BreakSTRU_HomeLevel _array_element)) _returnvalue_3)
          (bind _structout (Utilities|Struct|SetmembersinSTRU_HomeLevel _array_element true))
          (Utilities|Array|SetArrayElem _level_names _array_index _structout))))))

(fn ConstructionScript)