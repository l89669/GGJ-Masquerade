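; BP_Base_Grid is a base grid-cell actor that can display a number through a TextRender.
; The construction script and Tick both copy Number and ShowingNumber into the text and its visibility.
; On Visible and On Invisible toggle ShowingNumber, while On Passable, On Impassable and On Normal are empty hooks.
; An unused fallback for turning the text toward the player camera remains in the graph, disconnected.
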(event EventTick
  (params (DeltaSeconds :type Float%20%28single-precision%29))
  ;[0.15 0.15 0.15 0.5] 数据绑定
  (Utilities|FlowControl|Sequence
    (:then_0
      (Rendering|SetVisibility (Variables|Default|GetTextRender) (Variables|Default|GetbShowing%20Number) false)
      (Rendering|Components|TextRender|SetText (Variables|Default|GetTextRender) (Utilities|Text|ToText(Integer) (Variables|Default|GetNumber))))))

(fn ConstructionScript
  (Rendering|SetVisibility (Variables|Default|GetTextRender) (Variables|Default|GetbShowing%20Number) false)
  (Rendering|Components|TextRender|SetText (Variables|Default|GetTextRender) (Utilities|Text|ToText(Integer) (Variables|Default|GetNumber))))

(fn OnPassable)

(fn OnImpassable)

(fn OnNormal)

(fn OnVisible
  (Variables|Default|SetbShowing%20Number true))

(fn OnInvisible
  (Variables|Default|SetbShowing%20Number false))