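; BP_PropGrid is a prop actor whose mesh is chosen by prop type and which can be triggered a limited number of times.
; The construction script looks up the static mesh in a map, with a patch that enlarges the copper mesh.
; OnTrigger prints the remaining count, then returns false if none remain; otherwise it decrements, plays a sound, optionally hides the mesh when exhausted, and returns true.
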(event EventBeginPlay)

(event Collision|EventActorBeginOverlap
  (params (OtherActor :type Actor%20Object%20Reference)))

(event EventTick
  (params (DeltaSeconds :type Float%20%28single-precision%29))
  (|CallParentFunction DeltaSeconds) ; 此节点被禁用，将不会被调用。\n从引脚连出引线来编译功能。
)

(fn ConstructionScript
  (bind _prop_type (Variables|Default|GetProp%20Type))
  (bind _prop_mesh (Variables|Setting|GetProp%20Mesh))
  (bind _value (Utilities|Map|Find _prop_mesh _prop_type))
  ;[0.15 0.15 0.15 0.5] 根据道具类型设置静态网格体
  (Components|StaticMesh|SetStaticMesh (Variables|Default|GetPropMesh) _value)
  ;;[0.15 0.15 0.15 0.5] 补丁
  (if (== _value "/Game/Masquerade/Props/Grid/CopperMesh/SM_Copper.SM_Copper")
    (Transformation|SetWorldScale3D (Variables|Default|GetPropMesh) "3.000000,3.000000,3.000000"))
  (|CallParentFunction))

(fn OnTrigger
  (Utilities|FlowControl|Sequence
    (:then_0
      (Development|PrintString (Utilities|String|Append "剩余触发次数：" (Utilities|String|ToString(Integer) (Variables|Setting|GetTrigger%20Count)))) ; .DLP_
    )
    (:then_1
      ;[0.15 0.15 0.15 0.5] 是否让触发
      (if (<= (Variables|Setting|GetTrigger%20Count) 0)
        (return false)
        (else
          (Math|Integer|DecrementInt (Variables|Setting|GetTrigger%20Count)
            (:%20%20
              (Utilities|FlowControl|Sequence
                (:then_0
                  (Audio|PlaySound2D "/Game/Masquerade/Music/Prop/SW_Paperman.SW_Paperman" 1.0 1.0 0.0 0 0) ; .Mus_
                  ;[0.15 0.15 0.15 0.5] 触发后是否耗尽触发次数并隐藏网格
                  (if (and (<= (Variables|Setting|GetTrigger%20Count) 0) (Variables|Setting|GetbHide%20Mesh))
                    (Rendering|SetVisibility (Variables|Default|GetPropMesh) false false)))
                (:then_1
                  (return true))))))))))