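; Player controller for a mask-based grid puzzle: runs clicks, movement, level flow and player, dialog and favorites UI.
; A box trace around the current grid marks passable neighbors by the worn mask's number rule.
; Moves use SimpleMoveToLocation plus a timed delay, then spend steps or pretend points (restarting when both are empty) and resolve the grid.
; Grids swap mask pawns, trigger collectible stories saved to GameInstance, or end the level, gated by switch count.
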(event Custom|Move
  (params (Target%20Grid :type BP%20Base%20Grid%20Object%20Reference))
  (bind _calibrationpoint (Variables|/Game/Masquerade/Props/Grid/BP_Base_Grid.BP_Base_Grid_C|GetCalibrationPoint Target%20Grid))
  (bind _returnvalue (Transformation|GetWorldLocation _calibrationpoint))
  ;[0.15 0.15 0.15 0.5] 移动后刷新格子样式
  (if (not (Variables|Default|GetbMoving))
    (Variables|Default|SetbMoving true)
    (Variables|Local|SetTarget%20Grid Target%20Grid)
    ;;[0.15 0.15 0.15 0.5] 异步的AI Move To因未知原因不能使用，唯此下策
    (AI|Navigation|SimpleMovetoLocation self (+ _returnvalue (* (Math|Vector|Normalize (- _returnvalue (Transformation|GetWorldLocation (Variables|/Game/Masquerade/Props/Grid/BP_Base_Grid.BP_Base_Grid_C|GetCalibrationPoint (Variables|Default|GetCurrent%20Grid))))) (Components|Capsule|GetScaledCapsuleRadius (Variables|/Script/Engine.Character|GetCapsuleComponent (.AsBP%20Player (Utilities|Casting|CastToBP_Player (Pawn|GetControlledPawn))))) 1.1)))
    (Utilities|FlowControl|Sequence
      (:then_0
        (Utilities|FlowControl|Delay (+ (/ (Math|Vector|VectorLength (- (+ _returnvalue (* (Math|Vector|Normalize (- _returnvalue (Transformation|GetWorldLocation (Variables|/Game/Masquerade/Props/Grid/BP_Base_Grid.BP_Base_Grid_C|GetCalibrationPoint (Variables|Default|GetCurrent%20Grid))))) (Components|Capsule|GetScaledCapsuleRadius (Variables|/Script/Engine.Character|GetCapsuleComponent (.AsBP%20Player (Utilities|Casting|CastToBP_Player (Pawn|GetControlledPawn))))) 1.1)) (Transformation|GetActorLocation (Pawn|GetControlledPawn)))) 6e+02) 0.4))
        (bind _bdead (Grids|ReduceSteporPretend))
        (if _bdead
          ;;[0.15 0.15 0.15 0.5] 死亡重生
          (Grids|SwitchPlayerCharacter true "/Game/Masquerade/Characters/Player/BP_Player.BP_Player_C")
          (else
            (Variables|Default|SetCurrent%20Grid (Variables|Local|GetTarget%20Grid))
            ;;[0.15 0.15 0.15 0.5] 判定格子
            (Grids|DecideGrid (Variables|Default|GetCurrent%20Grid))
            (Grids|FlushViewFieldGrids)
            (Variables|Default|SetbMoving false)
            (Development|PrintString "已刷新视野") ; .DLP_
          ))))))

(event Input|EnhancedActionEvents|EnhancedInputActionIA_Restart
  (params (ActionValue :type Boolean) (ElapsedSeconds :type Float%20%28double-precision%29) (TriggeredSeconds :type Float%20%28double-precision%29) (InputAction :type Input%20Action%20Object%20Reference :default "/Game/Masquerade/Characters/Player/Input/Actions/IA_Restart.IA_Restart"))
  ;[0.15 0.15 0.15 0.5] 重新开始关卡
  (:Started
    (CallFunction|Restart)))

(event Input|EnhancedActionEvents|EnhancedInputActionIA_Click
  (params (ActionValue :type Boolean) (ElapsedSeconds :type Float%20%28double-precision%29) (TriggeredSeconds :type Float%20%28double-precision%29) (InputAction :type Input%20Action%20Object%20Reference :default "/Game/Masquerade/Characters/Player/Input/Actions/IA_Click.IA_Click"))
  (bind (_hit _hitactor) (Grids|GetLocationUnderCursor))
  ;[0.05098 0.05098 0.05098] 左键单击事件
  (:Started
    ;;[0.15 0.15 0.15 0] 点击判定
    (Utilities|FlowControl|Sequence
      (:then_0
        (if _hit
          (bind _asbp_base_grid (Utilities|Casting|CastToBP_Base_Grid _hitactor))
          (Default|OnClick _asbp_base_grid self)))
      (:then_1
        (Audio|PlaySound2D "/Game/Masquerade/Music/Interaction/SW_Click.SW_Click" 1.0 1.0 0.0 0 0) ; .Mus_
      ))))

(event EventBeginPlay
  (bind _returnvalue (PlayerController|LocalPlayerSubsystems|GetEnhancedInputLocalPlayerSubsystem))
  (bind _self self)
  (bind _self_2 self)
  (bind _self_3 self)
  (bind _self_4 self)
  (bind _self_5 self)
  ;[0.05098 0.05098 0.05098] 初始设置
  (|CallParentFunction) ; 暂时是空的
  (Utilities|FlowControl|Sequence
    (:then_0
      ;;[0.15 0.15 0.15 0.5] 留给关卡加载的缓冲时间
      (Input|DisableInput _self_4 _self_4)
      (CallFunction|SetEyeState false)
      (Utilities|FlowControl|Delay 1.0)
      (CallFunction|OpenEye false)
      (Input|EnableInput _self_5 _self_5))
    (:then_1
      ;;[0.15 0.15 0.15 0.5] 从游戏实例中获取纸人剧情配置
      (Variables|Setting|SetPaperman%20Setting (Variables|/Game/Masquerade/Core/BP_GI_Base.BP_GI_Base_C|GetPaperman%20Setting (CallFunction|GetGameInstance))))
    (:then_2
      ;;[0.15 0.15 0.15 0.5] 操作映射上下文
      (Utilities|FlowControl|Delay 1.0)
      (Utilities|IsValid _returnvalue
        (:Is%20Valid
          (Input|AddMappingContext _returnvalue "/Game/Masquerade/Characters/Player/Input/IMC_Player.IMC_Player" 0 "(bIgnoreAllPressedKeysUntilRelease=True,bForceImmediately=False,bNotifyUserSettings=False)"))))
    (:then_3
      ;;[0.15 0.15 0.15 0.5] 初始格子
      (bind _outactors (Actor|GetAllActorsOfClasswithTag "/Game/Masquerade/Props/Grid/BP_Base_Grid.BP_Base_Grid_C" "Initial"))
      (Variables|Default|SetCurrent%20Grid (Utilities|Array|Get(acopy) _outactors)))
    (:then_4
      ;;[0.15 0.15 0.15 0.5] 初始视野
      (Grids|FlushViewFieldGrids))
    (:then_5
      ;;[0.15 0.15 0.15 0.5] 玩家UI
      (bind _returnvalue_2 (UserInterface|CreateWidget "/Game/Masquerade/UI/WBP_Player.WBP_Player_C" _self _self))
      (UserInterface|Viewport|AddtoViewport _returnvalue_2 0)
      (Variables|Default|SetPlayer%20UI _returnvalue_2))
    (:then_6
      ;;[0.15 0.15 0.15 0.5] 对话框UI
      (bind _returnvalue_3 (UserInterface|CreateWidget "/Game/Masquerade/UI/WBP_DialogBox.WBP_DialogBox_C" _self_2 _self_2))
      (UserInterface|Viewport|AddtoViewport _returnvalue_3 0)
      (bind _output_get (Variables|Default|SetDialogBox%20UI _returnvalue_3))
      (Widget|SetVisibility _output_get "Collapsed"))
    (:then_7
      ;;[0.15 0.15 0.15 0.5] 根据当前关卡设置最大切换面具次数
      (Variables|Default|SetMax%20Mask%20Switch%20Count (.MaxSwitchMaskCount (Utilities|Struct|BreakSTRU_LevelSetting (CallFunction|GetCurrentLevelSetting)))))
    (:then_8
      ;;[0.15 0.15 0.15 0.5] 恢复输入模式
      (Input|SetInputModeGameandUI self 0 "DoNotLock" true false))
    (:then_9
      ;;[0.15 0.15 0.15 0.5] 设置字符串表ID
      (Variables|默认|SetFinish%20Text%20ST%20ID (.OutTableId (Class|KismetTextLibrary|StringTableIdandKeyfromText "Index"))))
    (:then_10
      ;;[0.15 0.15 0.15 0.5] 统计纸人道具数量
      (Variables|Default|SetMax%20Paperman%20Count 0)
      (bind _outactors_2 (Actor|GetAllActorsOfClass "/Game/Masquerade/Props/Grid/BP_PropGrid.BP_PropGrid_C"))
      (for _array_element _outactors_2
        (switch Utilities|FlowControl|Switch|SwitchonE_Prop (Variables|/Game/Masquerade/Props/Grid/BP_PropGrid.BP_PropGrid_C|GetProp%20Type _array_element)
          (:NewEnumerator0
            (Math|Integer|IncrementInt (Variables|Default|GetMax%20Paperman%20Count))))))
    (:then_11
      ;;[0.15 0.15 0.15 0.5] 防止卡视角问题
      (Utilities|FlowControl|Delay 0.2)
      (Utilities|Casting|CastToBP_Player (Pawn|GetControlledPawn)
        (:CastFailed
          (Grids|SwitchPlayerCharacter true "/Game/Masquerade/Characters/Player/BP_Player.BP_Player_C")
          (Utilities|FlowControl|Delay 0.6)
          (Utilities|Casting|CastToBP_Player (Pawn|GetControlledPawn)
            (:CastFailed
              (Grids|SwitchPlayerCharacter true "/Game/Masquerade/Characters/Player/BP_Player.BP_Player_C"))))))
    (:then_12
      ;;[0.15 0.15 0.15 0.5] 创建收藏夹控件
      (bind _returnvalue_4 (UserInterface|CreateWidget "/Game/Masquerade/UI/WBP_Favorite.WBP_Favorite_C" _self_3 _self_3 (Variables|默认|GetFinish%20Text%20ST%20ID)))
      (UserInterface|Viewport|AddtoViewport _returnvalue_4 0)
      (bind _output_get_2 (Variables|Default|SetFavorite%20UI _returnvalue_4))
      (Widget|SetVisibility _returnvalue_4 "Collapsed"))))

(event EventEndPlay
  (params (EndPlayReason :type EEndPlayReason%20Enum :default "Destroyed"))
  ;[0.15 0.15 0.15 0.5] 自动同步纸人剧情配置
  (Variables|/Game/Masquerade/Core/BP_GI_Base.BP_GI_Base_C|SetPaperman%20Setting (CallFunction|GetGameInstance) (Variables|Setting|GetPaperman%20Setting)))

(fn ConstructionScript)

(fn GetLocationUnderCursor
  (bind _hitresult (Game|Player|GetHitResultUnderCursorbyChannel "TraceTypeQuery3" true))
  (bind (_bblockinghit _binitialoverlap _time _distance _location _impactpoint _normal _impactnormal _physmat _hitactor) (Collision|BreakHitResult _hitresult))
  (return _bblockinghit _hitactor))

(fn FlushViewFieldGrids
  (bind _current_grid (Variables|Default|GetCurrent%20Grid))
  (bind _viewfield (Variables|Setting|GetViewField))
  (bind _calibrationpoint (Variables|/Game/Masquerade/Props/Grid/BP_Base_Grid.BP_Base_Grid_C|GetCalibrationPoint _current_grid))
  (bind _returnvalue (Transformation|GetWorldLocation _calibrationpoint))
  (bind _returnvalue_2 (- (.x _returnvalue) 275.0))
  (bind _returnvalue_3 (Math|Vector|MakeVector _returnvalue_2 (.y _returnvalue) (.z _returnvalue)))
  ;[0.15 0.15 0.15 0.5] 将之前的格子变为普通格子
  (Grids|CleanViewFieldGrids)
  ;[0.15 0.15 0.15 0.5] 寻找当前视野内的可通行与不可通行格子
  (bind _outhits (Class|KismetSystemLibrary|BoxTraceMulti _returnvalue_3 _returnvalue_3 (Math|Vector|MakeVector (- (* (.x _viewfield) 2.2e+02) 45.0) (- (* (.y _viewfield) 2.2e+02) 9e+01) 3e+02) "0, 0, 0" "TraceTypeQuery3" false 0 "None" true))
  (for _array_element _outhits
    (bind _asbp_base_grid (Utilities|Casting|CastToBP_Base_Grid (.HitActor (Collision|BreakHitResult _array_element))))
    (bind _output_get (LocalVariables|SetGrid _asbp_base_grid))
    ;[0.15 0.15 0.15 0.5] 格子可见
    (Default|OnVisible _output_get)
    ;[0.15 0.15 0.15 0.5] 不允许走相同数字的格子
    (if (!= (Variables|/Game/Masquerade/Props/Grid/BP_Base_Grid.BP_Base_Grid_C|GetNumber (LocalVariables|GetGrid)) (Variables|/Game/Masquerade/Props/Grid/BP_Base_Grid.BP_Base_Grid_C|GetNumber (Variables|Default|GetCurrent%20Grid)))
      ;[0.15 0.15 0.15 0.5] 判定格子是否可通行
      (switch Utilities|FlowControl|Switch|SwitchonE_MaskType (Variables|Default|GetCurrent%20Mask)
        (:NewEnumerator0
          (if (<= (Math|Integer|Absolute(Integer) (- (Variables|/Game/Masquerade/Props/Grid/BP_Base_Grid.BP_Base_Grid_C|GetNumber (LocalVariables|GetGrid)) (Variables|/Game/Masquerade/Props/Grid/BP_Base_Grid.BP_Base_Grid_C|GetNumber (Variables|Default|GetCurrent%20Grid)))) 1)
            ;;[0.15 0.15 0.15 0.5] 可以通行
            (Utilities|Set|Add (Variables|Default|GetPassable%20Grids) (LocalVariables|GetGrid) :!label _label)
            (Default|OnPassable (LocalVariables|GetGrid))
            (else
              ;;[0.15 0.15 0.15 0.5] 不可通行
              (Utilities|Set|Add (Variables|Default|GetImpassable%20Grids) (LocalVariables|GetGrid) :!label _label_2)
              (Default|OnImpassable (LocalVariables|GetGrid)))))
        (:NewEnumerator1
          (bind _bis_near (Grids|IsNearNumber (Variables|/Game/Masquerade/Props/Grid/BP_Base_Grid.BP_Base_Grid_C|GetNumber (Variables|Default|GetCurrent%20Grid)) false (Variables|/Game/Masquerade/Props/Grid/BP_Base_Grid.BP_Base_Grid_C|GetNumber (LocalVariables|GetGrid))))
          (if _bis_near
            (goto _label)
            (else
              (goto _label_2))))
        (:NewEnumerator2
          (bind _bis_near_2 (Grids|IsNearNumber (Variables|/Game/Masquerade/Props/Grid/BP_Base_Grid.BP_Base_Grid_C|GetNumber (Variables|Default|GetCurrent%20Grid)) true (Variables|/Game/Masquerade/Props/Grid/BP_Base_Grid.BP_Base_Grid_C|GetNumber (LocalVariables|GetGrid))))
          (if _bis_near_2
            (goto _label)
            (else
              (goto _label_2))))
        (:NewEnumerator3
          ;;[0.15 0.15 0.15 0.5] 初始无面具，仅可走唯一一步
          (bind _outactors (Actor|GetAllActorsOfClasswithTag "/Game/Masquerade/Props/Grid/BP_Base_Grid.BP_Base_Grid_C" "First"))
          (if (== (Utilities|Array|Get(acopy) _outactors) (LocalVariables|GetGrid))
            (Utilities|Set|Add (Variables|Default|GetPassable%20Grids) (LocalVariables|GetGrid))
            (Default|OnPassable (Utilities|Array|Get(acopy) _outactors))
            (else
              (Utilities|Set|Add (Variables|Default|GetImpassable%20Grids) (LocalVariables|GetGrid))
              (Default|OnImpassable (LocalVariables|GetGrid))))))
      (else
        ;[0.15 0.15 0.15 0.5] 不可通行
        (Utilities|Set|Add (Variables|Default|GetImpassable%20Grids) (LocalVariables|GetGrid))
        (Default|OnImpassable (LocalVariables|GetGrid))))))

(fn CleanViewFieldGrids
  (bind _impassable_grids (Variables|Default|GetImpassable%20Grids))
  (bind _passable_grids (Variables|Default|GetPassable%20Grids))
  (Utilities|FlowControl|Sequence
    (:then_0
      (bind _valuepin (Utilities|Set|ForEachLoop(Set) _passable_grids)
        (:then
          (Default|OnNormal _valuepin)
          (Default|OnInvisible _valuepin))
        (:CompletedPin
          (Utilities|Set|Clear _passable_grids))))
    (:then_1
      (bind _valuepin_2 (Utilities|Set|ForEachLoop(Set) _impassable_grids)
        (:then
          (Default|OnNormal _valuepin_2)
          (Default|OnInvisible _valuepin_2))
        (:CompletedPin
          (Utilities|Set|Clear _impassable_grids))))))

(fn ReduceSteporPretend
  (bind _player_ui (Variables|Default|GetPlayer%20UI))
  ;[0.15 0.15 0.15 0.5] 步数
  (if (> (Variables|Default|GetCurrent%20Step) 0)
    (Math|Integer|DecrementInt (Variables|Default|GetCurrent%20Step)
      (:%20%20
        _))
    (else
      ;[0.15 0.15 0.15 0.5] 伪装值
      (if (> (Variables|Default|GetCurrent%20Pretend) 0)
        (bind _result (Math|Integer|DecrementInt (Variables|Default|GetCurrent%20Pretend))
          (:%20%20
            (UserInterface|Animation|PlayAnimation _player_ui (Variables|/Game/Masquerade/UI/WBP_Player.WBP_Player_C|GetBreathe _player_ui) 0.0 1 "Forward" 1.0 false)
            (Audio|PlaySound2D "/Game/Masquerade/Music/Move/SW_Pretend_Low.SW_Pretend_Low" (* (Math|Conversions|ToFloat(Integer) (- 3 _result)) 2.5) 1.0 0.0 0 0) ; .Mus_
          ))
        (else
          (Development|PrintString "死亡") ; .DLP_
          (return true)))))
  (Utilities|FlowControl|Sequence
    (:then_0
      (Development|PrintString (Utilities|String|Append "当前步数：" (Utilities|String|ToString(Integer) (Variables|Default|GetCurrent%20Step)))) ; .DLP_
    )
    (:then_1
      (Development|PrintString (Utilities|String|Append "当前伪装值：" (Utilities|String|ToString(Integer) (Variables|Default|GetCurrent%20Pretend)))) ; .DLP_
    )
    (:then_2
      (return false))))

(fn DecideGrid
  (params (Grid :type BP%20Base%20Grid%20Object%20Reference))
  (bind _level_setting (CallFunction|GetCurrentLevelSetting))
  (bind _next_level_name (CallFunction|GetNextLevelName))
  (bind _game_instance (CallFunction|GetGameInstance))
  (bind _paperman_setting (Variables|Setting|GetPaperman%20Setting))
  (bind _returnvalue (Utilities|String|ToString(Name) (.levelname _level_setting)))
  (bind _forpeach_setting (Variables|/Game/Masquerade/Core/BP_GI_Base.BP_GI_Base_C|GetForPeach%20Setting _game_instance))
  (switch Utilities|FlowControl|Switch|SwitchonE_GridType (Variables|/Game/Masquerade/Props/Grid/BP_Base_Grid.BP_Base_Grid_C|GetType Grid)
    (:NewEnumerator0
      (return))
    (:NewEnumerator2
      ;[0.15 0.15 0.15 0.5] 供桃道具结算
      (Audio|PlaySound2D "/Game/Masquerade/Music/Move/SW_EndingLevel.SW_EndingLevel" 1.0 1.0 0.0 0 0)
      (if (<= (Variables|Default|GetMask%20Switch%20Count) (Variables|Default|GetMax%20Mask%20Switch%20Count))
        ;[0.15 0.15 0.15 0.5] 通过供桃判定，进入结局剧情
        (Utilities|FlowControl|Sequence
          (:then_0
            (Development|PrintString "通过供桃判定") ; .DLP_
          )
          (:then_1
            (Widget|RemovefromParent (Variables|Default|GetPlayer%20UI))
            (Variables|Default|SetPlayer%20UI 0)
            (Widget|RemovefromParent (Variables|Default|GetDialogBox%20UI))
            (Variables|Default|SetDialogBox%20UI 0)
            (Utilities|FlowControl|Sequence
              (:then_0
                ;;[0.15 0.15 0.15 0.5] 结局文案
                (bind _returnvalue_2 (UserInterface|CreateWidget "/Game/Masquerade/UI/WBP_FinishConversation.WBP_FinishConversation_C" self (Class|KismetStringTableLibrary|GetTableEntrySourceString (Variables|默认|GetFinish%20Text%20ST%20ID) (Utilities|String|ToString(Name) (.LevelName (Utilities|Struct|BreakSTRU_LevelSetting (CallFunction|GetCurrentLevelSetting))))) 0.01 (CallFunction|GetNextLevelName)))
                (UserInterface|Viewport|AddtoViewport _returnvalue_2 0)
                (Input|SetInputModeUIOnly self _returnvalue_2 "DoNotLock" false))
              (:then_1
                ;[0.15 0.15 0.15 0.5] 记录供桃剧情已触发
                (bind _structout (Utilities|Struct|SetmembersinSTRU_ForPeach_Setting (.Value (Utilities|Map|Find _forpeach_setting _returnvalue)) true))
                (Utilities|Map|Add _forpeach_setting _returnvalue _structout)
                (return)))))
        (else
          ;[0.15 0.15 0.15 0.5] 没有通过供桃判定，直接进入下一关
          (if (!= _next_level_name "")
            (Game|OpenLevel(byName) _next_level_name)
            (Development|PrintString "到达终点") ; .DLP_
            (return)
            (else
              ;;[0.15 0.15 0.15 0.5] TODO_：当最后一关没有通过供桃判定，进入游戏结束界面
              (Game|OpenLevel(byName) "LV_End_CG")
              (return))))))
    (:NewEnumerator3
      (Utilities|FlowControl|Sequence
        (:then_0
          ;[0.15 0.15 0.15 0.5] 面具
          (bind _asbp_mask_grid (Utilities|Casting|CastToBP_MaskGrid Grid))
          (Grids|SwitchMask (Variables|/Game/Masquerade/Props/Grid/BP_MaskGrid.BP_MaskGrid_C|GetMask%20Type _asbp_mask_grid))
          (Utilities|FlowControl|Sequence
            (:then_0
              (Development|PrintString (Utilities|String|Append "当前步数：" (Utilities|String|ToString(Integer) (Variables|Default|GetCurrent%20Step)))) ; .DLP_
            )
            (:then_1
              (Development|PrintString (Utilities|String|Append "当前伪装值：" (Utilities|String|ToString(Integer) (Variables|Default|GetCurrent%20Pretend)))) ; .DLP_
            )
            (:then_2
              (return))))
        (:then_1
          ;[0.15 0.15 0.15 0.5] 道具
          (bind _asbp_prop_grid (Utilities|Casting|CastToBP_PropGrid Grid))
          (bind _bcan_trigger (Default|OnTrigger _asbp_prop_grid))
          (if _bcan_trigger
            (switch Utilities|FlowControl|Switch|SwitchonE_Prop (Variables|/Game/Masquerade/Props/Grid/BP_PropGrid.BP_PropGrid_C|GetProp%20Type _asbp_prop_grid)
              (:NewEnumerator0
                (Utilities|FlowControl|Sequence
                  (:then_0
                    (Math|Integer|IncrementInt (Variables|Default|GetPaperman%20Count)))
                  (:then_1
                    ;[0.15 0.15 0.15 0.5] 设置其为已收集
                    (bind _structout_2 (Utilities|Struct|SetmembersinSTRU_Paperman_Setting (.Value (Utilities|Map|Find _paperman_setting (Variables|/Game/Masquerade/Props/Grid/BP_PropGrid.BP_PropGrid_C|GetProp%20Name _asbp_prop_grid))) true))
                    (Utilities|Map|Add _paperman_setting (Variables|/Game/Masquerade/Props/Grid/BP_PropGrid.BP_PropGrid_C|GetProp%20Name _asbp_prop_grid) _structout_2))
                  (:then_2
                    (Development|PrintString "进入供桃剧情") ; .DLP_
                  )
                  (:then_3
                    (Dialog|OnEntryStory (Variables|/Game/Masquerade/Props/Grid/BP_PropGrid.BP_PropGrid_C|GetProp%20Name _asbp_prop_grid)))
                  (:then_4
                    (return)))))))))))

(fn SwitchMask
  (params (Type :type E_MaskType%20Enum :default "NewEnumerator0"))
  (Math|Integer|IncrementInt (Variables|Default|GetMask%20Switch%20Count)
    (:%20%20
      (Variables|Default|SetCurrent%20Mask Type)
      (Variables|Default|SetCurrent%20Step (.Value (Utilities|Map|Find (Variables|Setting|GetMask%20Step) Type)))
      (Grids|SwitchPlayerCharacter false (.Value (Utilities|Map|Find (Variables|Setting|GetMask%20Mesh) Type)))
      (Utilities|FlowControl|Sequence
        (:then_0
          (Audio|PlaySound2D "/Game/Masquerade/Music/Prop/SW_Switch_Mask.SW_Switch_Mask" 1.0 1.0 0.0 0 0) ; .Mus_
        )
        (:then_1
          (switch Utilities|FlowControl|Switch|SwitchonE_MaskType (Variables|Default|GetCurrent%20Mask)
            (:NewEnumerator0
              (Audio|PlaySound2D "/Game/Masquerade/Music/Prop/SW_Mouse.SW_Mouse" 1.0 1.0 0.0 0 0) ; .Mus_
            )
            (:NewEnumerator1
              (Audio|PlaySound2D "/Game/Masquerade/Music/Prop/SW_Fox.SW_Fox" 1.0 1.0 0.0 0 0) ; .Mus_
            )
            (:NewEnumerator2
              (Audio|PlaySound2D "/Game/Masquerade/Music/Prop/SW_Ghost.SW_Ghost" 1.0 1.0 0.0 0 0) ; .Mus_
            )))
        (:then_2
          (Development|PrintString (Utilities|String|Append "当前面具：" (Utilities|String|EnumtoString Type))) ; .DLP_
        )))))

(fn SwitchPlayerCharacter
  (params (bRevive :type Boolean) (New%20Character :type BP%20Player%20Class%20Reference))
  (if bRevive
    (CallFunction|Restart)
    (else
      (AI|Navigation|StopMovement)
      (Variables|Local|SetPlayer%20Transform (Transformation|GetActorTransform (Pawn|GetControlledPawn)))
      (Actor|DestroyActor (Pawn|GetControlledPawn))
      (bind _returnvalue (Game|SpawnActorfromClass New%20Character (Variables|Local|GetPlayer%20Transform) "Undefined" "MultiplyWithRoot" 0 0))
      (Pawn|Possess _returnvalue))))

(fn IsNearNumber
  (params (Number :type Integer) (bOdd :type Boolean) (Target%20Number :type Integer))
  ;[0.15 0.15 0.15 0.5] 确定模数
  (if bOdd
    (LocalVariables|SetModulus 1)
    (else
      (LocalVariables|SetModulus 0)))
  ;[0.15 0.15 0.15 0.5] 是否相邻
  (if (<= (Math|Integer|Absolute(Integer) (- Target%20Number Number)) 2)
    ;[0.15 0.15 0.15 0.5] 是否是符合的奇/偶数
    (if (== (Math|Integer|%(Integer) Target%20Number 2) (LocalVariables|GetModulus))
      (return true)
      (else
        (return false)))
    (else
      (return false))))

(fn OnEntryStory
  (params (Prop%20Name :type Name))
  (Utilities|FlowControl|Sequence
    (:then_0
      (Widget|SetVisibility (Variables|Default|GetPlayer%20UI) "Collapsed")
      (Widget|SetVisibility (Variables|Default|GetFavorite%20UI) "Collapsed")
      (Widget|SetVisibility (Variables|Default|GetDialogBox%20UI) "Visible")
      (Input|SetInputModeUIOnly self 0 "DoNotLock" false))
    (:then_1
      (Default|EntryStory (Variables|Default|GetDialogBox%20UI) (.Section (Utilities|Struct|BreakSTRU_Paperman_Setting (.Value (Utilities|Map|Find (Variables|Setting|GetPaperman%20Setting) Prop%20Name)))) "\\r\\n"))))

(fn OnQuitStory
  (Widget|SetVisibility (Variables|Default|GetDialogBox%20UI) "Collapsed")
  (Widget|SetVisibility (Variables|Default|GetPlayer%20UI) "Collapsed")
  (Widget|SetVisibility (Variables|Default|GetPlayer%20UI) "Visible")
  (Input|SetInputModeGameandUI self 0 "DoNotLock" true false))

(fn IsPassibleGrid
  (params (Grid :type BP%20Base%20Grid%20Object%20Reference))
  (return (Utilities|Set|Contains (Variables|Default|GetPassable%20Grids) Grid)))

(fn GetCurrentLevelSetting
  (bind _returnvalue (Game|GetCurrentLevelName true))
  (if (.ReturnValue (Utilities|Map|Find (Variables|Setting|GetLevel%20Setting) _returnvalue))
    (return (.Value (Utilities|Map|Find (Variables|Setting|GetLevel%20Setting) _returnvalue)))
    (else
      (return ""))))

(fn GetNextLevelName
  (bind _level_setting (Variables|Setting|GetLevel%20Setting))
  (bind _returnvalue (Game|GetCurrentLevelName true))
  (bind _keys (Utilities|Map|Keys _level_setting))
  (for (_array_element _array_index) _keys
    (if (Utilities|Enum|Equal(Enum) _array_element _returnvalue)
      (return (Utilities|String|StringToName (.Key (Utilities|Map|GetKeyValueByIndex _level_setting (+ _array_index 1)))))))
  (return "None"))

(fn Restart
  (Utilities|FlowControl|Sequence
    (:then_0
      (Development|PrintString "重开关卡"))
    (:then_1
      (bind _returnvalue (Game|GetCurrentLevelName true))
      (Game|OpenLevel(byName) (Utilities|String|StringToName _returnvalue)))
    (:then_2
      (return))))

(fn OnEntryFavorite
  (Widget|SetVisibility (Variables|Default|GetPlayer%20UI) "Collapsed")
  (Widget|SetVisibility (Variables|Default|GetDialogBox%20UI) "Collapsed")
  (Widget|SetVisibility (Variables|Default|GetFavorite%20UI) "Visible")
  (Input|SetInputModeUIOnly self 0 "DoNotLock" false)
  (Default|FlushFavorite (Variables|Default|GetFavorite%20UI)))

(fn OnQuitFavorite
  (Widget|SetVisibility (Variables|Default|GetFavorite%20UI) "Collapsed")
  (Widget|SetVisibility (Variables|Default|GetDialogBox%20UI) "Collapsed")
  (Widget|SetVisibility (Variables|Default|GetPlayer%20UI) "Visible")
  (Input|SetInputModeGameandUI self 0 "DoNotLock" true false))